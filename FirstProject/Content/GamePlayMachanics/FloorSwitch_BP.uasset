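; FloorSwitch_BP is a floor switch actor that animates a door and the switch itself up and down.
; Raise and lower events play or reverse two timelines, one for the door and one for the switch.
; Timeline updates feed track values to UpdateDoorLocation and UpdateFloorSwitchLocation, which are defined outside this graph, as is the triggering logic.
; An unconnected node that would offset MPDoor upward never runs.
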(event `self.RaiseDoor`
  (bind (_direction `_새_트랙_0`) (`Timeline|DoorTimeLine` :`NewTime` (`GameplayStatics.GetWorldDeltaSeconds`) :!label _label)
    (:`Update`
      (`self.UpdateDoorLocation` `_새_트랙_0`))))

(event `self.LowerDoor`
  (goto _label :!via `Reverse`))

(event `self.RaiseFloorSwitch`
  (bind (_direction `_새_트랙_0`) (`Timeline|타임라인_0` :`NewTime` (`GameplayStatics.GetWorldDeltaSeconds`) :!label _label_2)
    (:`Update`
      (`self.UpdateFloorSwitchLocation` `_새_트랙_0`))))

(event `self.LowerFloorSwitch`
  (goto _label_2 :!via `Reverse`))

(fn `UserConstructionScript`)